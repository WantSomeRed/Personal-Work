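; Base weapon Blueprint that provides fire, fire-mode, reload and first-equip logic, with empty hook events for child weapons.
; BeginPlay caches the player character, sets the current fire mode and plays the first-equip montage.
; Fire plays a weapon montage and calls the hooks and OnFire dispatcher; Reload animates the character mesh.
; ChangeFireMode calls OnChangeFireMode directly or through Automatic and Burst timelines; timeline stop logic is unwired.
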(event `CE_OnFire`
  ;[1 1 1] Function for inheritance
)

(event `self.ReceiveBeginPlay`
  (bind _asue_4asp_character (cast `/Game/Ue4ASP_Character` (`GameplayStatics.GetPlayerCharacter` 0)))
  (set `self.Character` _asue_4asp_character)
  (set `self.CurrentFireMode` (`|GetArrayItem` (`self.FireMode`) (`self.FireModeIndex`)))
  (`|ExecutionSequence`
    (:`then_0`
      (if (`self.IsFirstEquipt`)
        (`|PlayMontage` (`self.WeaponMesh`) (`self.EquippedMontage`)
          (:`OnCompleted`
            (set `self.IsFirstEquipt` false)))))))

(event `CE_StopFire`
  ;[1 1 1] Function for inheritance
)

(event `/Game/Weapon/BPI_Gun.Fire`
  (`|PlayMontage` (`self.WeaponMesh`) (`self.FireMontage`)
    (:`then`
      (`self.CE_OnFire`)
      (`self.OnFire`)
      (`self.CE_StopFire`))))

(event `/Game/Weapon/BPI_Gun.ChangeFireMode`
  (`self.CE_OnFire`)
  (switch `/Game/Weapon/Enums/EFireMode` (`self.CurrentFireMode`)
    (:`NewEnumerator0`
      _)
    (:`NewEnumerator1`
      _)
    (:`NewEnumerator2`
      (`Timeline|AutoMatic`
        (:`Fire`
          _)))
    (:`NewEnumerator3`
      (`Timeline|Burst` :!via `PlayFromStart`
        (:`Burst fire`
          _))))
  (`self.OnChangeFireMode`))

(event `/Game/Weapon/BPI_Gun.Reload`
  (`|PlayMontage` (`Character.Mesh` (`self.Character`)) (`self.ReloadMontage`)))

(event `/Game/Weapon/BPI_Gun.Aimming`)

(fn `AddPlayerPitchAndYawInput`
  (params (Pitch :type "Float (double-precision)") (Yaw :type "Float (double-precision)"))
  (bind _character (`self.Character`))
  (`/Engine/EditorBlueprintResources/StandardMacros.IsValid` (`self.Character`)
    (:`Is Valid`
      (`Pawn.AddControllerPitchInput` _character Pitch)
      (`Pawn.AddControllerYawInput` _character Yaw))))

(fn `FireModeSwitch`
  (switch `/Game/Weapon/Enums/EFireMode` (`self.CurrentFireMode`)
    (:`NewEnumerator0`
      (set `self.CurrentFireMode` "NewEnumerator0"))
    (:`NewEnumerator1`
      (set `self.CurrentFireMode` "NewEnumerator1"))
    (:`NewEnumerator2`
      (set `self.CurrentFireMode` "NewEnumerator2"))
    (:`NewEnumerator3`
      (set `self.CurrentFireMode` "NewEnumerator3"))))

(fn `UserConstructionScript`)