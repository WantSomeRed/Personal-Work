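; M4 weapon Blueprint that applies camera recoil while firing and pulls the aim back when firing stops.
; Firing plays RecoilTimeline forward, feeding its pitch and randomized yaw curves into player look input.
; Stopping reverses the timeline at higher speed with negated input for recovery.
; That recovery is scaled by the pitch difference between control rotations captured once at fire start and recovery start, relative to RecoilMaxThreshold.
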(event `self.CE_OnFire`
  (bind (_returnvalue_roll _returnvalue_pitch) (`KismetMathLibrary.BreakRotator` (`KismetMathLibrary.NormalizedDeltaRotator` (`self.OriginRotation`) (`self.PostRecoilRotation`))))
  (bind _returnvalue (`KismetMathLibrary.Abs` _returnvalue_pitch))
  (bind _returnvalue_2 (select `bool` (> _returnvalue (`self.RecoilMaxThreshold`)) :`false` (`KismetMathLibrary.MapRangeClamped` _returnvalue 0.0 (`self.RecoilMaxThreshold`) 0.0 1.0) :`true` (`KismetMathLibrary.MapRangeClamped` _returnvalue (`self.RecoilMaxThreshold`) 30.0 1.0)))
  (`TimelineComponent.SetPlayRate` (`self.RecoilTimeline`) 1.0)
  (`|ExecutionSequence`
    (:`then_0`
      (`/Engine/EditorBlueprintResources/StandardMacros.DoOnce` false :!label _label
        (:`Completed`
          (set `self.OriginRotation` (`Controller.GetControlRotation` (`GameplayStatics.GetPlayerController` 0))))))
    (:`then_1`
      (bind (_direction _pitch _yaw) (`Timeline|RecoilTimeline` :!label _label_2)
        (:`Update`
          (switch `ETimelineDirection` _direction
            (:`Forward`
              (`self.AddPlayerPitchAndYawInput` _pitch (* _yaw (`KismetMathLibrary.RandomFloatInRange` 0.3 1.0))))
            (:`Backward`
              (`|ExecutionSequence`
                (:`then_0`
                  (`/Engine/EditorBlueprintResources/StandardMacros.DoOnce` false :!label _label_3
                    (:`Completed`
                      (set `self.PostRecoilRotation` (`Controller.GetControlRotation` (`GameplayStatics.GetPlayerController` 0))))))
                (:`then_1`
                  (`self.AddPlayerPitchAndYawInput` (* _pitch -12.0 _returnvalue_2) (* _yaw -3.0 _returnvalue_2)))))))
        (:`Finished`
          (switch `ETimelineDirection` _direction
            (:`Forward`
              (`self.CE_ResetRecoil`))))))))

(event `CE_ResetRecoil`
  (`|ExecutionSequence`
    (:`then_0`
      (goto _label :!via `Reset`))
    (:`then_1`
      (goto _label_3 :!via `Reset`))))

(event `self.CE_StopFire`
  (`TimelineComponent.SetPlayRate` (`self.RecoilTimeline`) 12.0)
  (goto _label_2 :!via `Reverse`))

(fn `UserConstructionScript`
  (`parent.UserConstructionScript`))